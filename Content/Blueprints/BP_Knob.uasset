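; BP_Knob is a rotatable knob actor that a finger pinch turns around its yaw axis.
; A pinch attaches RotateTarget to the given component, keeping world transform, and opens a Tick gate; stopping interaction detaches it and closes the gate.
; While open, Tick copies RotateTarget's actor-relative yaw to RotationOrigin, zeroing pitch and roll, so the knob follows only the twist.
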(event Custom|OnFingerPinched
  (params (AttachTarget :type Primitive%20Component%20Object%20Reference))
  (Transformation|AttachComponentToComponent (Variables|Default|GetRotateTarget) AttachTarget "None" "KeepWorld" "KeepWorld" "KeepWorld" true)
  (Utilities|FlowControl|Gate true) ; enters at Open
)

(event Custom|OnInteractionStopped
  (Transformation|DetachFromComponent (Variables|Default|GetRotateTarget) "KeepWorld" "KeepWorld" "KeepWorld" true)
  (Utilities|FlowControl|Gate true) ; enters at Close
)

(event EventTick
  (params (DeltaSeconds :type Float%20%28single-precision%29))
  (Utilities|FlowControl|Gate true
    (:Exit
      (Transformation|SetRelativeRotation (Variables|Default|GetRotationOrigin) (Math|Rotator|MakeRotator 0.0 0.0 (.Yaw (Math|Rotator|BreakRotator (.Rotation (Math|Transform|BreakTransform (Math|Transform|MakeRelativeTransform (Transformation|GetWorldTransform (Variables|Default|GetRotateTarget)) (Transformation|GetActorTransform))))))) false false))))

(fn ConstructionScript)